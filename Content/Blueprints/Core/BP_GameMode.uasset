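; Game mode that acts as the central manager for UI screens, menu navigation and streamed level loading.
; Once the game instance is ready, it creates hidden widgets from its screen list and stores them in a settings map.
; ShowScreen and HideScreen read that map to drive fades, pausing, input mode, cursor and level unloading.
; LoadLevel fades in a loading screen, streaming the level when that animation finishes, then fades out.
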(event EventBeginPlay
  (CallFunction|MainSetup))

(event Custom|InitializeUI
  (UserInterface|InitializeUILoopScreens :!label _label)
  (UserInterface|InitializeUICheckScreens)
  (if (not (Variables|Default|GetUI_Widgets_OK))
    (Utilities|FlowControl|Delay 0.2)
    (goto _label)))

(event Custom|MainSetup
  (bind _asbp_game_instance (Utilities|Casting|CastToBP_GameInstance (Game|GetGameInstance))
    (:then
      (bind _output_get (Variables|References|SetGameInstance_Ref _asbp_game_instance))
      (Utilities|IsValid _output_get
        (:Is%20Valid
          (Utilities|FlowControl|Delay 0.2)
          (CallFunction|InitializeUI))
        (:Is%20Not%20Valid
          (Utilities|Time|SetTimerbyEvent (delegate Custom|MainSetup) 0.2 :!label _label))))
    (:CastFailed
      (goto _label))))

(event Custom|FadeInLoadingGame
  (Default|Fadein (Variables|UserInterface|GetUI_LoadingGame_Ref)))

(event Custom|FadeOutLoadingGame
  (Utilities|FlowControl|Delay (Variables|UserInterface|GetUI_FadeDelay))
  (Default|FadeOut (Variables|UserInterface|GetUI_LoadingGame_Ref)))

(event Custom|ShowScreen
  (params (ScreenName :type ENUM_Screens%20Enum :default "NewEnumerator0"))
  (bind _returnvalue (Utilities|String|EnumtoString ScreenName))
  (bind _screensinfolist (Variables|Default|GetScreensInfoList))
  (bind _returnvalue_2 (Utilities|String|StringToName _returnvalue))
  (bind (_value _returnvalue_3) (Utilities|Map|Find _screensinfolist _returnvalue_2))
  (bind (_showfadein _hidescreensbefore _unloadlevel _delaybeforefadein _showmousecursorfadein _pausegameonshow _widget _inputmodefadein) (Utilities|Struct|BreakSTRUCT_UI_Info _value))
  (bind _asui_base_menu (Utilities|Casting|CastToUI_Base_Menu _widget))
  (if _returnvalue_3
    (Variables|Default|SetCurrentScreen ScreenName)
    (Variables|Default|SetCurrent_UI_Widget _widget)
    (Variables|Default|SetCurrentScreenInfo _value)
    (if _hidescreensbefore
      (UIScreens|HideScreens))
    (if _unloadlevel
      (CallFunction|UnloadLevel))
    (if _delaybeforefadein
      (Utilities|FlowControl|Delay (Variables|UserInterface|GetUI_FadeDelay)))
    (if _showfadein
      (Default|Fadein _asui_base_menu))
    (UserInterface|SetScreenInputMode _inputmodefadein _asui_base_menu)
    (Variables|/Script/Engine.PlayerController|SetbShowMouseCursor (Game|GetPlayerController 0) _showmousecursorfadein)
    (CallFunction|RebuildNavigationMenu)
    ;[1 1 1] Pause Game on Show
    (if _pausegameonshow
      (Game|SetGamePaused true))
    (else
      (Development|PrintString (Utilities|String|Append "ERROR: SCREEN NOT FOUND -> " (Utilities|String|EnumtoString ScreenName)) true true "(R=1.000000,G=0.000000,B=0.000000,A=1.000000)" 2e+01))))

(event Custom|FadeInLoadingLevel
  (Default|Fadein (Variables|UserInterface|GetUI_LoadingLevel_Ref)))

(event Custom|FadeOutLoadingLevel
  (Utilities|FlowControl|Delay (Variables|UserInterface|GetUI_FadeDelay))
  (Default|FadeOut (Variables|UserInterface|GetUI_LoadingLevel_Ref)))

(event Custom|RebuildNavigationMenu
  (Default|UpdateCurrentInputVisualization (.AsBP%20Player%20Controller (Utilities|Casting|CastToBP_PlayerController (Game|GetPlayerController 0)))))

(event Custom|LoadLevel
  (params (LevelName :type ENUM_Maps%20Enum :default "NewEnumerator0"))
  (Variables|Default|SetCurrentLevel LevelName)
  (CallFunction|FadeinLoadingLevel)
  (EventDispatchers|BindEventtoFadeAnimationFinished (Variables|UserInterface|GetUI_LoadingLevel_Ref) (delegate Custom|LoadingProcess))
  (UIScreens|HideScreens))

(event Custom|LoadingProcess
  (bind _currentlevel (Variables|Default|GetCurrentLevel))
  (bind _returnvalue (Utilities|String|EnumtoString _currentlevel))
  (bind _returnvalue_2 (Utilities|String|StringToName _returnvalue))
  (Game|LoadStreamLevel(byName) _returnvalue_2 true)
  (EventDispatchers|UnbindEventfromFadeAnimationFinished (Variables|UserInterface|GetUI_LoadingLevel_Ref) (delegate Custom|LoadingProcess))
  (Utilities|FlowControl|Delay (Variables|UserInterface|GetUI_FadeDelay))
  (Class|BPIBaseLevel|SetupLevel(Message) (Class|GameplayStatics|GetStreamingLevel _returnvalue_2))
  (CallFunction|FadeOutLoadingLevel))

(event Custom|UnloadLevel
  (if (Utilities|Enum|NotEqual(Enum) (Variables|Default|GetMainLevel) (Variables|Default|GetCurrentLevel))
    (Game|UnloadStreamLevel(byName) (Utilities|String|StringToName (Utilities|String|EnumtoString (Variables|Default|GetCurrentLevel))) false)
    (Variables|Default|SetCurrentLevel (Variables|Default|GetMainLevel))))

(event Custom|LoadSlot
  (params (SlotNum :type Integer))
  (CallFunction|LoadLevel "NewEnumerator4"))

(event Custom|MainMenu_Start
  (CallFunction|GotoSelectLevel))

(event Custom|MainMenu_Quit
  (Game|QuitGame 0 "Quit" false))

(event Custom|MainMenu_Credits
  (CallFunction|ShowScreen "NewEnumerator4"))

(event Custom|MainMenu_Options
  (CallFunction|ShowScreen "NewEnumerator3"))

(event Custom|Gameplay_PauseGame
  (if (not (Game|IsGamePaused))
    (CallFunction|ShowScreen "NewEnumerator5")))

(event Custom|Goto_SelectLevel
  (CallFunction|ShowScreen "NewEnumerator7"))

(event Custom|Goto_Gameplay
  (CallFunction|ShowScreen "NewEnumerator6"))

(event Custom|Goto_MainMenu
  (CallFunction|ShowScreen "NewEnumerator2"))

(fn ConstructionScript)

(fn InitializeUILoopScreens
  (for _array_element (Variables|/Game/Blueprints/Core/BP_GameInstance.BP_GameInstance_C|GetScreensArray (Variables|References|GetGameInstance_Ref))
    (LocalVariables|SetScreenNameEnum _array_element)
    (LocalVariables|SetScreenName (Utilities|String|StringToName (Utilities|String|EnumtoString _array_element)))
    (switch Utilities|FlowControl|Switch|SwitchonENUM_Screens _array_element
      (:NewEnumerator0
        (UserInterface|InitializeUILoadingGame))
      (:NewEnumerator1
        (UserInterface|InitializeUILoadingLevel))
      (:NewEnumerator2
        (bind _outputpin (UserInterface|InitializeUIMainMenu))
        (LocalVariables|SetNewWidget _outputpin)
        (Variables|/Game/UI/BaseUI/UI_Base_Menu.UI_Base_Menu_C|SetScreenNameEnum (LocalVariables|GetNewWidget) (LocalVariables|GetScreenNameEnum) :!label _label)
        (Variables|/Game/UI/BaseUI/UI_Base_Menu.UI_Base_Menu_C|SetScreenName (LocalVariables|GetNewWidget) (LocalVariables|GetScreenName))
        (Utilities|Array|Add (Variables|Default|GetUI_Widgets) (LocalVariables|GetNewWidget))
        (UserInterface|SetupScreensInfoList (LocalVariables|GetScreenName) (LocalVariables|GetNewWidget)))
      (:NewEnumerator3
        (bind _widget (UserInterface|InitializeUIOptions))
        (LocalVariables|SetNewWidget _widget)
        (goto _label))
      (:NewEnumerator7
        (bind _outputpin_2 (UserInterface|InitializeUISelectLevel))
        (LocalVariables|SetNewWidget _outputpin_2)
        (goto _label))
      (:NewEnumerator4
        (bind _outputpin_3 (UserInterface|InitializeUICredits))
        (LocalVariables|SetNewWidget _outputpin_3)
        (goto _label))
      (:NewEnumerator5
        (bind _outputpin_4 (UserInterface|InitializeUIPauseMenu))
        (LocalVariables|SetNewWidget _outputpin_4)
        (goto _label))
      (:NewEnumerator6
        (bind _outputpin_5 (UserInterface|InitializeUIGameplay))
        (LocalVariables|SetNewWidget _outputpin_5)
        (goto _label))
      (:NewEnumerator8
        (bind _outputpin_6 (UserInterface|InitializeUILevelCompleted))
        (LocalVariables|SetNewWidget _outputpin_6)
        (goto _label))
      (:NewEnumerator9
        (bind _outputpin_7 (UserInterface|InitializeUIPlayerDied))
        (LocalVariables|SetNewWidget _outputpin_7))))
  (return))

(fn InitializeUICheckScreens
  (Variables|Default|SetUI_Widgets_OK true)
  (for _array_element (Variables|Default|GetUI_Widgets)
    (Utilities|IsValid _array_element
      (:Is%20Not%20Valid
        (Variables|Default|SetUI_Widgets_OK false))))
  (return))

(fn InitializeUILoadingGame
  (bind _returnvalue (UserInterface|CreateWidget "/Game/UI/Loading/UI_LoadingGame.UI_LoadingGame_C"))
  (bind _output_get (Variables|UserInterface|SetUI_LoadingGame_Ref _returnvalue))
  (Widget|SetVisibility _output_get "Hidden")
  (UserInterface|Viewport|AddtoViewport _output_get 0))

(fn InitializeUILoadingLevel
  (bind _returnvalue (UserInterface|CreateWidget "/Game/UI/Loading/UI_LoadingLevel.UI_LoadingLevel_C"))
  (bind _output_get (Variables|UserInterface|SetUI_LoadingLevel_Ref _returnvalue))
  (Widget|SetVisibility _output_get "Hidden")
  (UserInterface|Viewport|AddtoViewport _output_get 0))

(fn InitializeUIMainMenu
  (bind _returnvalue (UserInterface|CreateWidget "/Game/UI/Screens/UI_MainMenu.UI_MainMenu_C"))
  (bind _output_get (Variables|UserInterface|SetUI_MainMenu_Ref _returnvalue))
  (Widget|SetVisibility _output_get "Hidden")
  (UserInterface|Viewport|AddtoViewport _output_get 0)
  (return _output_get))

(fn InitializeUIOptions
  (bind _returnvalue (UserInterface|CreateWidget "/Game/UI/Screens/UI_Options.UI_Options_C"))
  (bind _output_get (Variables|UserInterface|SetUI_Options_Ref _returnvalue))
  (Widget|SetVisibility _output_get "Hidden")
  (UserInterface|Viewport|AddtoViewport _output_get 0)
  (Variables|/Game/UI/BaseUI/UI_Base_Menu.UI_Base_Menu_C|SetScreenName _output_get (Utilities|String|StringToName (Utilities|String|EnumtoString (Utilities|Enum|LiteralenumENUM_Screens "NewEnumerator3"))))
  (Utilities|Array|Add (Variables|Default|GetUI_Widgets) _output_get)
  (return _output_get))

(fn InitializeUICredits
  (bind _returnvalue (UserInterface|CreateWidget "/Game/UI/Screens/UI_Credits.UI_Credits_C"))
  (bind _output_get (Variables|UserInterface|SetUI_Credits_Ref _returnvalue))
  (Widget|SetVisibility _output_get "Hidden")
  (UserInterface|Viewport|AddtoViewport _output_get 0)
  (return _output_get))

(fn InitializeUIGameplay
  (bind _returnvalue (UserInterface|CreateWidget "/Game/UI/Screens/UI_Gameplay.UI_Gameplay_C"))
  (bind _output_get (Variables|UserInterface|SetUI_Gameplay_Ref _returnvalue))
  (Widget|SetVisibility _output_get "Hidden")
  (UserInterface|Viewport|AddtoViewport _output_get 0)
  (return _output_get))

(fn HideScreen
  (params (ScreenNameEnum :type ENUM_Screens%20Enum :default "NewEnumerator0") (ScreenName :type Name))
  (if (== ScreenName "")
    (LocalVariables|SetHideScreenName (Utilities|String|StringToName (Utilities|String|EnumtoString ScreenNameEnum)))
    (else
      (LocalVariables|SetHideScreenName ScreenName)))
  (if (.ReturnValue (Utilities|Map|Find (Variables|Default|GetScreensInfoList) (LocalVariables|GetHideScreenName)))
    (bind _asui_base_menu (Utilities|Casting|CastToUI_Base_Menu (.Widget (Utilities|Struct|BreakSTRUCT_UI_Info (.Value (Utilities|Map|Find (Variables|Default|GetScreensInfoList) (LocalVariables|GetHideScreenName))))))
      (:then
        (LocalVariables|SetCurrentWidget _asui_base_menu)
        (if (.ShowFadeOut (Utilities|Struct|BreakSTRUCT_UI_Info (.Value (Utilities|Map|Find (Variables|Default|GetScreensInfoList) (LocalVariables|GetHideScreenName)))))
          (if (Widget|IsVisible (LocalVariables|GetCurrentWidget))
            (Default|FadeOut (LocalVariables|GetCurrentWidget))))
        (UserInterface|SetScreenInputMode (.InputModeFadeOut (Utilities|Struct|BreakSTRUCT_UI_Info (.Value (Utilities|Map|Find (Variables|Default|GetScreensInfoList) (LocalVariables|GetHideScreenName))))) (LocalVariables|GetCurrentWidget))
        (Variables|/Script/Engine.PlayerController|SetbShowMouseCursor (Game|GetPlayerController 0) (.ShowMouseCursorFadeOut (Utilities|Struct|BreakSTRUCT_UI_Info (.Value (Utilities|Map|Find (Variables|Default|GetScreensInfoList) (LocalVariables|GetHideScreenName))))))
        (if (.UnpauseGameOnHide (Utilities|Struct|BreakSTRUCT_UI_Info (.Value (Utilities|Map|Find (Variables|Default|GetScreensInfoList) (LocalVariables|GetHideScreenName)))))
          (Game|SetGamePaused false)))
      (:CastFailed
        (Development|PrintString (Utilities|String|Append "ERROR: Can't find screen REFERENCE in Dictionary -> " (Utilities|String|ToString(Name) (LocalVariables|GetHideScreenName))))))
    (else
      (Development|PrintString (Utilities|String|Append "ERROR: Can't find screen ITEM in Dictionary -> " (Utilities|String|ToString(Name) (LocalVariables|GetHideScreenName)))))))

(fn InitializeUIPauseMenu
  (bind _returnvalue (UserInterface|CreateWidget "/Game/UI/Screens/UI_PauseMenu.UI_PauseMenu_C"))
  (bind _output_get (Variables|UserInterface|SetUI_PauseMenu_Ref _returnvalue))
  (Widget|SetVisibility _output_get "Hidden")
  (UserInterface|Viewport|AddtoViewport _output_get 0)
  (return _output_get))

(fn InitializeUISelectLevel
  (bind _returnvalue (UserInterface|CreateWidget "/Game/UI/Screens/UI_SelectLevel.UI_SelectLevel_C"))
  (bind _output_get (Variables|UserInterface|SetUI_SelectLevel_Ref _returnvalue))
  (Widget|SetVisibility _output_get "Hidden")
  (UserInterface|Viewport|AddtoViewport _output_get 0)
  (return _output_get))

(fn InitializeUILevelCompleted
  (bind _returnvalue (UserInterface|CreateWidget "/Game/UI/Screens/UI_LevelCompleted.UI_LevelCompleted_C"))
  (bind _output_get (Variables|UserInterface|SetUI_LevelCompleted_Ref _returnvalue))
  (Widget|SetVisibility _output_get "Hidden")
  (UserInterface|Viewport|AddtoViewport _output_get 0)
  (return _output_get))

(fn InitializeUIPlayerDied
  (bind _returnvalue (UserInterface|CreateWidget "/Game/UI/Screens/UI_PlayerDied.UI_PlayerDied_C"))
  (bind _output_get (Variables|UserInterface|SetUI_PlayerDied_Ref _returnvalue))
  (Widget|SetVisibility _output_get "Hidden")
  (UserInterface|Viewport|AddtoViewport _output_get 0)
  (return _output_get))

(fn HideScreens
  (for _array_element (Variables|Default|GetUI_Widgets)
    (bind _asui_base_menu (Utilities|Casting|CastToUI_Base_Menu _array_element)
      (:then
        (UIScreens|HideScreen (Variables|/Game/UI/BaseUI/UI_Base_Menu.UI_Base_Menu_C|GetScreenNameEnum _asui_base_menu) (Variables|/Game/UI/BaseUI/UI_Base_Menu.UI_Base_Menu_C|GetScreenName _asui_base_menu)))
      (:CastFailed
        (Development|PrintString (Utilities|String|Append "ERROR: Can't find screen reference in Array-> " (Utilities|GetDisplayName _array_element)))))))

(fn SetScreenInputMode
  (params (InputMode :type ENUM_InputModes%20Enum :default "NewEnumerator0") (ScreenWidget :type UI%20Base%20Menu%20Object%20Reference))
  (bind _returnvalue (Game|GetPlayerController 0))
  (switch Utilities|FlowControl|Switch|SwitchonENUM_InputModes InputMode
    (:NewEnumerator3
      _)
    (:NewEnumerator0
      (Input|SetInputModeGameOnly _returnvalue))
    (:NewEnumerator1
      (Input|SetInputModeUIOnly _returnvalue ScreenWidget "DoNotLock"))
    (:NewEnumerator2
      (Input|SetInputModeGameandUI _returnvalue ScreenWidget "DoNotLock" true)))
  (return))

(fn SetupScreensInfoList
  (params (ScreenName :type Name) (Widget :type UI%20Base%20Menu%20Object%20Reference))
  (bind _screensinfolist (Variables|Default|GetScreensInfoList))
  (bind _value (Utilities|Map|Find _screensinfolist ScreenName))
  (bind (_showfadein _showfadeout _hidescreensbefore _unloadlevel _delaybeforefadein _showmousecursorfadein _showmousecursorfadeout _pausegameonshow _unpausegameonhide _widget _inputmodefadein) (Utilities|Struct|BreakSTRUCT_UI_Info _value))
  (Utilities|Map|Add (Variables|Default|GetScreensInfoList) ScreenName (Utilities|Struct|MakeSTRUCT_UI_Info _showfadein _showfadeout _hidescreensbefore _unloadlevel _delaybeforefadein _showmousecursorfadein false _pausegameonshow _unpausegameonhide Widget _inputmodefadein)))

(fn UpdateUIInputVisualization
  (bind _returnvalue (Game|GetPlayerController 0))
  (bind _currentscreeninfo (Variables|Default|GetCurrentScreenInfo))
  (bind (_widget _inputmodefadein) (Utilities|Struct|BreakSTRUCT_UI_Info _currentscreeninfo))
  (bind _asui_base_menu (Utilities|Casting|CastToUI_Base_Menu _widget))
  (UserInterface|SetScreenInputMode _inputmodefadein _asui_base_menu)
  (switch Utilities|FlowControl|Switch|SwitchonENUM_Controls (Variables|/Game/Blueprints/Core/BP_PlayerController.BP_PlayerController_C|GetCurrentControls (.AsBP%20Player%20Controller (Utilities|Casting|CastToBP_PlayerController (Game|GetPlayerController 0))))
    (:NewEnumerator0
      (Variables|/Script/Engine.PlayerController|SetbShowMouseCursor _returnvalue true :!label _label))
    (:NewEnumerator1
      (goto _label))
    (:NewEnumerator2
      (Variables|/Script/Engine.PlayerController|SetbShowMouseCursor _returnvalue false))))