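; Player controller that routes menu input to the current UI and tracks whether the player is using mouse, keyboard or gamepad.
; Menu actions navigate, select or cancel on the game mode's current UI_Base_Menu widget, while MenuShow asks the game mode to pause.
; Mouse position changes and gamepad-versus-keyboard key checks switch the active control scheme.
; Each switch refreshes the game mode's input visualization, redraws menu navigation and prints the current input.
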(event Custom|UpdateCurrentInputVisualization
  (bind _gamemode_ref (Variables|References|GetGameMode_Ref))
  (bind _current_ui_widget (Variables|/Game/Blueprints/Core/BP_GameMode.BP_GameMode_C|GetCurrent_UI_Widget _gamemode_ref))
  (bind (_asui_base_menu _bsuccess) (Utilities|Casting|CastToUI_Base_Menu _current_ui_widget))
  ;[1 1 1] Check Active Input
  (Default|UpdateUIInputVisualization _gamemode_ref)
  (if _bsuccess
    (Default|RedrawNavigation _asui_base_menu)))

(event EventBeginPlay
  (Variables|References|SetGameMode_Ref (.AsBP%20Game%20Mode (Utilities|Casting|CastToBP_GameMode (Game|GetGameMode))))
  (Variables|References|SetPlayerCharacter_Ref (.AsBP%20Player%20Character (Utilities|Casting|CastToBP_PlayerCharacter (Game|GetPlayerCharacter 0)))))

(event Input|ActionEvents|InputActionMenuDown
  (params (Key :type Key%20Structure :default "None"))
  (bind _gamemode_ref (Variables|References|GetGameMode_Ref))
  (bind _current_ui_widget (Variables|/Game/Blueprints/Core/BP_GameMode.BP_GameMode_C|GetCurrent_UI_Widget _gamemode_ref))
  (bind _asui_base_menu (Utilities|Casting|CastToUI_Base_Menu _current_ui_widget))
  (:Pressed
    (Default|NextNavButton _asui_base_menu)
    (Default|RedrawNavigation _asui_base_menu)))

(event Input|ActionEvents|InputActionMenuShow
  (params (Key :type Key%20Structure :default "None"))
  (:Pressed
    (Default|GameplayPauseGame (Variables|References|GetGameMode_Ref))))

(event Input|ActionEvents|InputActionMenuUp
  (params (Key :type Key%20Structure :default "None"))
  (bind _gamemode_ref (Variables|References|GetGameMode_Ref))
  (bind _current_ui_widget (Variables|/Game/Blueprints/Core/BP_GameMode.BP_GameMode_C|GetCurrent_UI_Widget _gamemode_ref))
  (bind _asui_base_menu (Utilities|Casting|CastToUI_Base_Menu _current_ui_widget))
  (:Pressed
    (Default|PreviousNavButton _asui_base_menu)
    (Default|RedrawNavigation _asui_base_menu)))

(event Input|ActionEvents|InputActionMenuSelect
  (params (Key :type Key%20Structure :default "None"))
  (:Pressed
    (Default|ClickCurrentButton (.AsUI%20Base%20Menu (Utilities|Casting|CastToUI_Base_Menu (Variables|/Game/Blueprints/Core/BP_GameMode.BP_GameMode_C|GetCurrent_UI_Widget (Variables|References|GetGameMode_Ref)))))))

(event Input|ActionEvents|InputActionSetKeyboard
  (params (Key :type Key%20Structure :default "None"))
  ;[1 1 1] Check Active Input
  (:Pressed
    (if (Class|KismetInputLibrary|KeyIsGamepadKey Key)
      (if (Utilities|Enum|NotEqual(Enum) (Variables|CheckControllers|GetCurrentControls) "NewEnumerator2")
        (Variables|CheckControllers|SetCurrentControls "NewEnumerator2")
        (CallFunction|UpdateCurrentInputVisualization :!label _label)
        (Development|PrintString (Utilities|String|Append "Current Input: " (Utilities|String|EnumtoString (Variables|CheckControllers|GetCurrentControls)))))
      (elif (Utilities|Enum|NotEqual(Enum) (Variables|CheckControllers|GetCurrentControls) "NewEnumerator1")
        (Variables|CheckControllers|SetCurrentControls "NewEnumerator1")
        (goto _label)))))

(event Input|ActionEvents|InputActionMenuCancel
  (params (Key :type Key%20Structure :default "None"))
  (:Pressed
    (Default|ClickCancelButton (.AsUI%20Base%20Menu (Utilities|Casting|CastToUI_Base_Menu (Variables|/Game/Blueprints/Core/BP_GameMode.BP_GameMode_C|GetCurrent_UI_Widget (Variables|References|GetGameMode_Ref)))))))

(event Input|AxisEvents|InputAxisMouseMovement
  (params (AxisValue :type Float%20%28single-precision%29))
  ;[1 1 1] Check Active Input
  (bind _isnewmouseevent (CallFunction|CheckChangedMouseInput))
  (if _isnewmouseevent
    (Variables|CheckControllers|SetCurrentControls "NewEnumerator0")
    (CallFunction|UpdateCurrentInputVisualization)
    (Development|PrintString (Utilities|String|Append "Current Input: " (Utilities|String|EnumtoString (Variables|CheckControllers|GetCurrentControls))))))

(fn ConstructionScript)

(fn CheckChangedMouseInput
  (bind _returnvalue (Game|GetPlayerController 0))
  (bind (_locationx _locationy) (Game|Player|GetMousePosition _returnvalue))
  (bind _returnvalue_2 (Math|Vector2D|MakeVector2D _locationx _locationy))
  (if (Class|KismetMathLibrary|NotEqualExactlyVector2DVector2D _returnvalue_2 (Variables|Default|GetLastMousePosition))
    (Variables|Default|SetLastMousePosition _returnvalue_2)
    (if (Utilities|Enum|Equal(Enum) (Variables|CheckControllers|GetCurrentControls) "NewEnumerator0")
      (LocalVariables|SetIsNewEvent false)
      (else
        (LocalVariables|SetIsNewEvent true)))
    (else
      (LocalVariables|SetIsNewEvent false)))
  (return (LocalVariables|GetIsNewEvent)))